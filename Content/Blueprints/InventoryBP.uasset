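; Inventory Blueprint that stores items in a Backpack array of bags, each holding an array of slot structs with ItemID and Durability.
; AddItem_Event writes to the given slot, or searches the bag for the first empty one (ItemID 0) when Slot is negative.
; RemoveItem_Event clears a slot by writing a zeroed struct.
; Both events print debug messages, and the construction script only prints a loading message.
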(event `RemoveItem_Event`
  (params (BagNumber :type Integer) (Slot :type Integer))
  (`KismetArrayLibrary.Array_Set` (`.Inventory_10_CB1BB80F4009C3D6D6C1539FC2C99391` (break `/Game/Blueprints/Structures/BackpackStructure` (`|GetArrayItem` (`self.Backpack`) BagNumber))) Slot (make `/Game/Blueprints/Structures/DragSlotStructure` 0))
  (`KismetSystemLibrary.PrintString` (`KismetStringLibrary.Concat_StrStr` "Removed item from bag " (`KismetStringLibrary.Conv_IntToString` BagNumber) ", slot " (`KismetStringLibrary.Conv_IntToString` Slot))))

(event `AddItem_Event`
  (params (Item :type "/Game/Blueprints/Structures/DragSlotStructure Structure") (BagNumber :type Integer) (Slot :type Integer))
  (bind (_number _slots _inventory) (break `/Game/Blueprints/Structures/BackpackStructure` (`|GetArrayItem` (`self.Backpack`) BagNumber)))
  (if (>= Slot 0)
    (`KismetArrayLibrary.Array_Set` _inventory Slot Item)
    (else
      (`KismetSystemLibrary.PrintString` "Finding first empty slot")
      (for (_array_element _array_index) _inventory
        (if (== (`.ItemID_2_DA5B4E834833CCBC19C3D5B72EE66724` (break `/Game/Blueprints/Structures/DragSlotStructure` _array_element)) 0)
          (break)))
      (`KismetArrayLibrary.Array_Set` _inventory _array_index Item)))
  (`KismetSystemLibrary.PrintString` (`KismetStringLibrary.Concat_StrStr` "Added Item " (`KismetStringLibrary.Conv_IntToString` (`.ItemID_2_DA5B4E834833CCBC19C3D5B72EE66724` (break `/Game/Blueprints/Structures/DragSlotStructure` Item))) " to bag " (`KismetStringLibrary.Conv_IntToString` 0) ", slot " (`KismetStringLibrary.Conv_IntToString` Slot))))

(fn `UserConstructionScript`
  (`KismetSystemLibrary.PrintString` "Loading Items"))
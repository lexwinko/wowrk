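; Character Blueprint that stores worn gear in an Equipment structure and prints a debug message when its sprite is clicked.
; Add and Remove events map a slot name to a struct member through long branch chains, writing the item or a zeroed drag slot.
; Both chains cross Shoulders and Neck, each writing the other's member.
; The CharacterDataTable lookup that would load Equipment by CharacterID is disconnected and never runs.
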(event `self.Sprite.OnClicked`
  (params (TouchedActor :type "Actor Object Reference") (ButtonPressed :type "Key Structure"))
  (`KismetSystemLibrary.PrintString` "Pressed Sprite"))

(event `AddEquipment_Event`
  (params (Item :type "/Game/Blueprints/Structures/DragSlotStructure Structure") (Slot :type String))
  (bind _equipment (`self.Equipment`))
  (`KismetSystemLibrary.PrintString` (`KismetStringLibrary.Concat_StrStr` "Adding  equipment id " (`KismetStringLibrary.Conv_IntToString` (`.ItemID_2_DA5B4E834833CCBC19C3D5B72EE66724` (break `/Game/Blueprints/Structures/DragSlotStructure` Item))) " to " Slot))
  (if (`KismetStringLibrary.EqualEqual_StrStr` Slot "Mainhand")
    (setmembers `/Game/Blueprints/Structures/EquipmentStructure` :`StructRef` _equipment :`Mainhand` Item)
    (`KismetSystemLibrary.PrintString` "Mainhand added succesfully")
    (elif (`KismetStringLibrary.EqualEqual_StrStr` Slot "Offhand")
      (setmembers `/Game/Blueprints/Structures/EquipmentStructure` :`StructRef` _equipment :`Offhand` Item)
      (elif (`KismetStringLibrary.EqualEqual_StrStr` Slot "Ranged")
        (setmembers `/Game/Blueprints/Structures/EquipmentStructure` :`StructRef` _equipment :`Ranged` Item)
        (elif (`KismetStringLibrary.EqualEqual_StrStr` Slot "Ammo")
          (setmembers `/Game/Blueprints/Structures/EquipmentStructure` :`StructRef` _equipment :`Ammo` Item)
          (elif (`KismetStringLibrary.EqualEqual_StrStr` Slot "Head")
            (setmembers `/Game/Blueprints/Structures/EquipmentStructure` :`StructRef` _equipment :`Head` Item)
            (elif (`KismetStringLibrary.EqualEqual_StrStr` Slot "Shoulders")
              (setmembers `/Game/Blueprints/Structures/EquipmentStructure` :`StructRef` _equipment :`Neck` Item)
              (elif (`KismetStringLibrary.EqualEqual_StrStr` Slot "Neck")
                (setmembers `/Game/Blueprints/Structures/EquipmentStructure` :`StructRef` _equipment :`Shoulder` Item)
                (elif (`KismetStringLibrary.EqualEqual_StrStr` Slot "Back")
                  (setmembers `/Game/Blueprints/Structures/EquipmentStructure` :`StructRef` _equipment :`Back` Item)
                  (elif (`KismetStringLibrary.EqualEqual_StrStr` Slot "Chest")
                    (setmembers `/Game/Blueprints/Structures/EquipmentStructure` :`StructRef` _equipment :`Chest` Item)
                    (elif (`KismetStringLibrary.EqualEqual_StrStr` Slot "Shirt")
                      (setmembers `/Game/Blueprints/Structures/EquipmentStructure` :`StructRef` _equipment :`Shirt` Item)
                      (elif (`KismetStringLibrary.EqualEqual_StrStr` Slot "Tabard")
                        (setmembers `/Game/Blueprints/Structures/EquipmentStructure` :`StructRef` _equipment :`Tabard` Item)
                        (elif (`KismetStringLibrary.EqualEqual_StrStr` Slot "Wrists")
                          (setmembers `/Game/Blueprints/Structures/EquipmentStructure` :`StructRef` _equipment :`Wrists` Item)
                          (elif (`KismetStringLibrary.EqualEqual_StrStr` Slot "Hands")
                            (setmembers `/Game/Blueprints/Structures/EquipmentStructure` :`StructRef` _equipment :`Hands` Item)
                            (elif (`KismetStringLibrary.EqualEqual_StrStr` Slot "Waist")
                              (setmembers `/Game/Blueprints/Structures/EquipmentStructure` :`StructRef` _equipment :`Waist` Item)
                              (elif (`KismetStringLibrary.EqualEqual_StrStr` Slot "Legs")
                                (setmembers `/Game/Blueprints/Structures/EquipmentStructure` :`StructRef` _equipment :`Legs` Item)
                                (elif (`KismetStringLibrary.EqualEqual_StrStr` Slot "Feet")
                                  (setmembers `/Game/Blueprints/Structures/EquipmentStructure` :`StructRef` _equipment :`Feet` Item)
                                  (elif (`KismetStringLibrary.EqualEqual_StrStr` Slot "FingerL")
                                    (setmembers `/Game/Blueprints/Structures/EquipmentStructure` :`StructRef` _equipment :`FingerL` Item)
                                    (elif (`KismetStringLibrary.EqualEqual_StrStr` Slot "FingerR")
                                      (setmembers `/Game/Blueprints/Structures/EquipmentStructure` :`StructRef` _equipment :`FingerR` Item)
                                      (elif (`KismetStringLibrary.EqualEqual_StrStr` Slot "TrinketL")
                                        (setmembers `/Game/Blueprints/Structures/EquipmentStructure` :`StructRef` _equipment :`TrinketL` Item)
                                        (elif (`KismetStringLibrary.EqualEqual_StrStr` Slot "TrinketR")
                                          (setmembers `/Game/Blueprints/Structures/EquipmentStructure` :`StructRef` _equipment :`TrinketR` Item))))))))))))))))))))))

(event `RemoveEquipment_Event`
  (params (Slot :type String))
  (bind _dragslotstructure (make `/Game/Blueprints/Structures/DragSlotStructure` 0))
  (bind _equipment (`self.Equipment`))
  (`KismetSystemLibrary.PrintString` (`KismetStringLibrary.Concat_StrStr` "Removed  equipment at " Slot))
  (if (`KismetStringLibrary.EqualEqual_StrStr` Slot "Mainhand")
    (setmembers `/Game/Blueprints/Structures/EquipmentStructure` :`StructRef` _equipment :`Mainhand` _dragslotstructure)
    (`KismetSystemLibrary.PrintString` "Mainhand removed succesfully")
    (elif (`KismetStringLibrary.EqualEqual_StrStr` Slot "Offhand")
      (setmembers `/Game/Blueprints/Structures/EquipmentStructure` :`StructRef` _equipment :`Offhand` _dragslotstructure)
      (elif (`KismetStringLibrary.EqualEqual_StrStr` Slot "Ranged")
        (setmembers `/Game/Blueprints/Structures/EquipmentStructure` :`StructRef` _equipment :`Ranged` _dragslotstructure)
        (elif (`KismetStringLibrary.EqualEqual_StrStr` Slot "Ammo")
          (setmembers `/Game/Blueprints/Structures/EquipmentStructure` :`StructRef` _equipment :`Ammo` _dragslotstructure)
          (elif (`KismetStringLibrary.EqualEqual_StrStr` Slot "Head")
            (setmembers `/Game/Blueprints/Structures/EquipmentStructure` :`StructRef` _equipment :`Head` _dragslotstructure)
            (elif (`KismetStringLibrary.EqualEqual_StrStr` Slot "Shoulders")
              (setmembers `/Game/Blueprints/Structures/EquipmentStructure` :`StructRef` _equipment :`Neck` _dragslotstructure)
              (elif (`KismetStringLibrary.EqualEqual_StrStr` Slot "Neck")
                (setmembers `/Game/Blueprints/Structures/EquipmentStructure` :`StructRef` _equipment :`Shoulder` _dragslotstructure)
                (elif (`KismetStringLibrary.EqualEqual_StrStr` Slot "Back")
                  (setmembers `/Game/Blueprints/Structures/EquipmentStructure` :`StructRef` _equipment :`Back` _dragslotstructure)
                  (elif (`KismetStringLibrary.EqualEqual_StrStr` Slot "Chest")
                    (setmembers `/Game/Blueprints/Structures/EquipmentStructure` :`StructRef` _equipment :`Chest` _dragslotstructure)
                    (elif (`KismetStringLibrary.EqualEqual_StrStr` Slot "Shirt")
                      (setmembers `/Game/Blueprints/Structures/EquipmentStructure` :`StructRef` _equipment :`Shirt` _dragslotstructure)
                      (elif (`KismetStringLibrary.EqualEqual_StrStr` Slot "Tabard")
                        (setmembers `/Game/Blueprints/Structures/EquipmentStructure` :`StructRef` _equipment :`Tabard` _dragslotstructure)
                        (elif (`KismetStringLibrary.EqualEqual_StrStr` Slot "Wrists")
                          (setmembers `/Game/Blueprints/Structures/EquipmentStructure` :`StructRef` _equipment :`Wrists` _dragslotstructure)
                          (elif (`KismetStringLibrary.EqualEqual_StrStr` Slot "Hands")
                            (setmembers `/Game/Blueprints/Structures/EquipmentStructure` :`StructRef` _equipment :`Hands` _dragslotstructure)
                            (elif (`KismetStringLibrary.EqualEqual_StrStr` Slot "Waist")
                              (setmembers `/Game/Blueprints/Structures/EquipmentStructure` :`StructRef` _equipment :`Waist` _dragslotstructure)
                              (elif (`KismetStringLibrary.EqualEqual_StrStr` Slot "Legs")
                                (setmembers `/Game/Blueprints/Structures/EquipmentStructure` :`StructRef` _equipment :`Legs` _dragslotstructure)
                                (elif (`KismetStringLibrary.EqualEqual_StrStr` Slot "Feet")
                                  (setmembers `/Game/Blueprints/Structures/EquipmentStructure` :`StructRef` _equipment :`Feet` _dragslotstructure)
                                  (elif (`KismetStringLibrary.EqualEqual_StrStr` Slot "FingerL")
                                    (setmembers `/Game/Blueprints/Structures/EquipmentStructure` :`StructRef` _equipment :`FingerL` _dragslotstructure)
                                    (elif (`KismetStringLibrary.EqualEqual_StrStr` Slot "FingerR")
                                      (setmembers `/Game/Blueprints/Structures/EquipmentStructure` :`StructRef` _equipment :`FingerR` _dragslotstructure)
                                      (elif (`KismetStringLibrary.EqualEqual_StrStr` Slot "TrinketL")
                                        (setmembers `/Game/Blueprints/Structures/EquipmentStructure` :`StructRef` _equipment :`TrinketL` _dragslotstructure)
                                        (elif (`KismetStringLibrary.EqualEqual_StrStr` Slot "TrinketR")
                                          (setmembers `/Game/Blueprints/Structures/EquipmentStructure` :`StructRef` _equipment :`TrinketR` _dragslotstructure))))))))))))))))))))))

(fn `UserConstructionScript`)